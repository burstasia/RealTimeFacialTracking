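; BP_GLENN is a test Blueprint that pulls face-tracking points from an external native DLL.
; On BeginPlay it loads DLLTestAgain.dll, binds its init and point-return functions in sequence, starts the tracker and stores the first points.
; Every Tick it refreshes the Points array, without checking that loading succeeded, and prints each element to screen.
; A failed DLL load feeds into that same element print node.
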(event EventBeginPlay
  (bind _returnvalue (Class|LinkDLL|ImportDLL "DLLs" "DLLTestAgain.dll"))
  (if _returnvalue
    (Development|PrintString "eyy")
    (bind _returnvalue_2 (Class|LinkDLL|ImportMethodInitFaceTracker))
    (if _returnvalue_2
      (Class|LinkDLL|InitFaceTracker)
      (bind _returnvalue_3 (Class|LinkDLL|ImportMethodReturnTrackedPoints))
      (if _returnvalue_3
        (bind _pointsreturn (Class|LinkDLL|ReturnTrackedPointsfromDLLArray))
        (Variables|Default|Setpoints _pointsreturn)))
    (else
      (Development|PrintString (Utilities|String|ToString(Vector2d) (stale EventTick _array_element))))))

(event EventTick
  (params (DeltaSeconds :type Float%20%28single-precision%29))
  (bind _pointsreturn (Class|LinkDLL|ReturnTrackedPointsfromDLLArray))
  (bind _output_get (Variables|Default|Setpoints _pointsreturn))
  (for _array_element _output_get
    (Development|PrintString (Utilities|String|ToString(Vector2d) _array_element))))

(fn ConstructionScript)