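; Test Blueprint that drives facial morph targets on a skeletal mesh from tracked 2D face points.
; Calibration stores neutral, exaggerated, smile and frown captures, and each FeatureList entry takes its X or Y range from neutral to its surprised, angry or happy pose.
; SetExpression offsets neutral positions by point 28's movement, then sets each morph weight as the clamped displacement divided by that range.
; Distance-based variants and a brow function are left unconnected.
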(event Custom|GetNeutralFace
  (params (TrackedNeutral :type Array%20of%20Vector%202D%20Structures))
  (bind _featurelist (Variables|Default|GetfeatureList))
  (bind _output_get (Variables|Default|SetneutralFace TrackedNeutral))
  (Variables|Default|SetposNeutralMidFace (Utilities|Array|Get(acopy) _output_get 28))
  (for (_array_element _array_index) _featurelist
    (Utilities|Array|SetArrayElem _featurelist _array_index (Utilities|Struct|MakeFeatureInfoStruct (.maxDistanceApart (Utilities|Struct|BreakFeatureInfoStruct _array_element)) (Utilities|Array|Get(acopy) (Variables|Default|GetneutralFace) (.indexFeature (Utilities|Struct|BreakFeatureInfoStruct _array_element))) (.isY (Utilities|Struct|BreakFeatureInfoStruct _array_element)) (.morphTargetName (Utilities|Struct|BreakFeatureInfoStruct _array_element)) (.indexFeature (Utilities|Struct|BreakFeatureInfoStruct _array_element)) (.arrayEnum (Utilities|Struct|BreakFeatureInfoStruct _array_element))))))

(event Custom|GetExaggeratedFace
  (params (Tracked%20Exaggerated :type Array%20of%20Vector%202D%20Structures))
  (bind _output_get (Variables|Default|SetexaggeratedFace Tracked%20Exaggerated))
  (Variables|Default|SetpreviousTrackedPoints _output_get))

(event Custom|GetSmileFace
  (params (Tracked%20Smile :type Array%20of%20Vector%202D%20Structures))
  (Variables|Default|SetsmileFace Tracked%20Smile))

(event Custom|GetFrownFace
  (params (TrackedFrown :type Array%20of%20Vector%202D%20Structures))
  (Variables|Default|SetfrownFace TrackedFrown))

(event Custom|SetMaxMin
  (for (_array_element _array_index) (Variables|Default|GetfeatureList)
    (CallFunction|CalculateMinMax _array_element _array_index)))

(event Custom|SetExpression
  (params (CurrentTrackedPoints :type Array%20of%20Vector%202D%20Structures))
  (Variables|Default|SettranslationNeutral (- (Utilities|Array|Get(acopy) CurrentTrackedPoints 28) (Variables|Default|GetposNeutralMidFace)))
  (for _array_element (Variables|Default|GetfeatureList)
    (if (.isY (Utilities|Struct|BreakFeatureInfoStruct _array_element))
      (Variables|Default|Setvalue (Math|Float|Clamp(Float) (/ (- (.Y (Math|Vector2D|BreakVector2D (+ (.posNeutral (Utilities|Struct|BreakFeatureInfoStruct _array_element)) (Variables|Default|GettranslationNeutral)))) (.y (Utilities|Array|Get(acopy) CurrentTrackedPoints (.indexFeature (Utilities|Struct|BreakFeatureInfoStruct _array_element))))) (.maxDistanceApart (Utilities|Struct|BreakFeatureInfoStruct _array_element)))))
      (else
        (Variables|Default|Setvalue (Math|Float|Clamp(Float) (/ (- (.X (Math|Vector2D|BreakVector2D (+ (.posNeutral (Utilities|Struct|BreakFeatureInfoStruct _array_element)) (Variables|Default|GettranslationNeutral)))) (.x (Utilities|Array|Get(acopy) CurrentTrackedPoints (.indexFeature (Utilities|Struct|BreakFeatureInfoStruct _array_element))))) (.maxDistanceApart (Utilities|Struct|BreakFeatureInfoStruct _array_element)))))))
    (Components|SkeletalMesh|SetMorphTarget (Variables|Default|GetSkeletalMesh) (.morphTargetName (Utilities|Struct|BreakFeatureInfoStruct _array_element)) (Variables|Default|Getvalue) true)))

(fn ConstructionScript)

(fn BrowSurprised
  (params (featureStruct :type Feature%20Info%20Struct%20Structure) (index :type Integer)))

(fn CalculateMinMax
  (params (featureInfo :type Feature%20Info%20Struct%20Structure) (arrayIndex :type Integer))
  (bind (_maxdistanceapart _posneutral _isy _morphtargetname _indexfeature _arrayenum) (Utilities|Struct|BreakFeatureInfoStruct featureInfo))
  (LocalVariables|SetindexFeature _indexfeature)
  (LocalVariables|SetposNeutral _posneutral)
  (switch Utilities|FlowControl|Switch|SwitchonarrayEnum _arrayenum
    (:NewEnumerator0
      (if _isy
        (LocalVariables|SetmaxDistance (- (.y (LocalVariables|GetposNeutral)) (.y (Utilities|Array|Get(acopy) (Variables|Default|GetexaggeratedFace) (LocalVariables|GetindexFeature)))))
        (else
          (LocalVariables|SetmaxDistance (- (.x (LocalVariables|GetposNeutral)) (.x (Utilities|Array|Get(acopy) (Variables|Default|GetexaggeratedFace) (LocalVariables|GetindexFeature))))))))
    (:NewEnumerator1
      (if _isy
        (LocalVariables|SetmaxDistance (- (.y (LocalVariables|GetposNeutral)) (.y (Utilities|Array|Get(acopy) (Variables|Default|GetfrownFace) (LocalVariables|GetindexFeature)))))
        (else
          (LocalVariables|SetmaxDistance (- (.x (LocalVariables|GetposNeutral)) (.x (Utilities|Array|Get(acopy) (Variables|Default|GetfrownFace) (LocalVariables|GetindexFeature))))))))
    (:NewEnumerator2
      (if _isy
        (LocalVariables|SetmaxDistance (- (.y (LocalVariables|GetposNeutral)) (.y (Utilities|Array|Get(acopy) (Variables|Default|GetsmileFace) (LocalVariables|GetindexFeature)))))
        (else
          (LocalVariables|SetmaxDistance (- (.x (LocalVariables|GetposNeutral)) (.x (Utilities|Array|Get(acopy) (Variables|Default|GetsmileFace) (LocalVariables|GetindexFeature)))))))))
  (Utilities|Array|SetArrayElem (Variables|Default|GetfeatureList) arrayIndex (Utilities|Struct|MakeFeatureInfoStruct (LocalVariables|GetmaxDistance) (LocalVariables|GetposNeutral) _isy _morphtargetname (LocalVariables|GetindexFeature) _arrayenum)))

(fn CalculateMaxDistance
  (params (points :type Array%20of%20Vector%202D%20Structures) (NewParam1 :type Boolean)))