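; Loads an external face-tracking DLL and uses its tracked points to drive facial expressions on an AnimActor.
; BeginPlay imports and initialises the tracker, then runs a timed, on-screen prompted calibration capturing neutral, frown, smile, surprised and closed-eye poses for the AnimActor.
; Once calibrated, Tick streams live points into SetFacialExpression.
; A disconnected debug branch would draw each captured pose as coloured circles.
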(event Custom|CalibrateNeutralFace
  (bind _pointsreturn (Class|LinkDLL|ReturnTrackedPointsfromDLLArray))
  (bind _output_get (Variables|Default|SetneutralFacePoints _pointsreturn))
  (Class|FaceAnimations|SetNeutralFace (Variables|Default|GetanimActor) _output_get))

(event Custom|CalibrateExaggeratedFace
  (bind _pointsreturn (Class|LinkDLL|ReturnTrackedPointsfromDLLArray))
  (bind _output_get (Variables|Default|SetexaggeratedFace _pointsreturn))
  (Class|FaceAnimations|SetSurprisedFace (Variables|Default|GetanimActor) _output_get))

(event Custom|CalibrateSmileFace
  (bind _pointsreturn (Class|LinkDLL|ReturnTrackedPointsfromDLLArray))
  (bind _output_get (Variables|Default|SetsmileFacePoints _pointsreturn))
  (Class|FaceAnimations|SetSmileFace (Variables|Default|GetanimActor) _output_get))

(event Custom|CalibrateFrownFace
  (bind _pointsreturn (Class|LinkDLL|ReturnTrackedPointsfromDLLArray))
  (bind _output_get (Variables|Default|SetfrownFacePoints _pointsreturn))
  (Class|FaceAnimations|SetAngryFace (Variables|Default|GetanimActor) _output_get))

(event Custom|CalibrateClosed
  (bind _pointsreturn (Class|LinkDLL|ReturnTrackedPointsfromDLLArray))
  (bind _output_get (Variables|Default|SetclosedFacePoints _pointsreturn))
  (Class|FaceAnimations|SetClosedEyes (Variables|Default|GetanimActor) _output_get))

(event EventBeginPlay
  (bind _returnvalue (Class|LinkDLL|ImportDLL "DLLs" "DLLTestAgain.dll"))
  (if _returnvalue
    (bind _returnvalue_2 (Class|LinkDLL|ImportMethodInitFaceTracker))
    (if _returnvalue_2
      (Class|LinkDLL|InitFaceTracker)
      (bind _returnvalue_3 (Class|LinkDLL|ImportMethodReturnTrackedPoints))
      (if _returnvalue_3
        (bind _pointsreturn (Class|LinkDLL|ReturnTrackedPointsfromDLLArray))
        (Variables|Default|Setpoints _pointsreturn)
        (Development|PrintString "Neutral" true true "(R=0.000000,G=0.660000,B=1.000000,A=1.000000)" 3.0)
        (Utilities|FlowControl|Delay 3.0)
        (CallFunction|CalibrateNeutralFace)
        (Development|PrintString "Frown" true true "(R=0.000000,G=0.660000,B=1.000000,A=1.000000)" 3.0)
        (Utilities|FlowControl|Delay 3.0)
        (CallFunction|CalibrateFrownFace)
        (Development|PrintString "Smile" true true "(R=0.000000,G=0.660000,B=1.000000,A=1.000000)" 3.0)
        (Utilities|FlowControl|Delay 3.0)
        (CallFunction|CalibrateSmileFace)
        (Development|PrintString "Surprised" true true "(R=0.000000,G=0.660000,B=1.000000,A=1.000000)" 3.0)
        (Utilities|FlowControl|Delay 3.0)
        (CallFunction|CalibrateExaggeratedFace)
        (Development|PrintString "Closed" true true "(R=0.000000,G=0.660000,B=1.000000,A=1.000000)" 3.0)
        (Utilities|FlowControl|Delay 3.0)
        (CallFunction|CalibrateClosed)
        (Class|FaceAnimations|SetMinMax (Variables|Default|GetanimActor))
        (Variables|Default|SetcalibrationDone true)))))

(event EventTick
  (params (DeltaSeconds :type Float%20%28single-precision%29))
  (if (Variables|Default|GetcalibrationDone)
    (bind _pointsreturn (Class|LinkDLL|ReturnTrackedPointsfromDLLArray))
    (Class|FaceAnimations|SetFacialExpression (Variables|Default|GetanimActor) _pointsreturn)))

(fn ConstructionScript)